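; Base fade actor for world cosmetics that gradually fades its mesh out and back in, such as climbable stairs.
; Construction caches original materials and creates dynamic instances of the masked fade materials.
; FadeOut swaps those in and plays a timeline driving their Fade parameter, which Fadein reverses.
; When the timeline finishes, full opacity restores original materials and blocking, while near-zero opacity ignores the cursor trace channel and, optionally, Visibility.
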(event `self.ReceiveBeginPlay`
  ;[0 1 0.1562] This Sets The Default Collision For Fully Visible
  (`self.Handle Collision` 1.0))

(event `/Game/Blueprints/Interfaces/BPI_Fade.Fade Out`
  ;[0.2656 0 1] Gradually Fade Out / Fade In
  (`self.Set Materials To Dynamic Instances`) ; This switches the materials from OG \nmaterials to Fade Materials, so that \nthey are masked instead of opaque and\nhave the fade parameter in them
  (bind (_direction _fade_alpha) (`Timeline|Fade` :`NewTime` 0.5 :!label _label)
    (:`Update`
      (for _array_element (`self.Dynamic Material Instances`)
        (`MaterialInstanceDynamic.SetScalarParameterValue` _array_element "Fade" _fade_alpha)))
    (:`Finished`
      (`self.Try To Reset Materials + Collision` _fade_alpha)
      (`self.Handle Collision` _fade_alpha))))

(event `/Game/Blueprints/Interfaces/BPI_Fade.Fade In`
  ;[0.2656 0 1] Gradually Fade Out / Fade In
  (goto _label :!via `Reverse`))

(event `Try To Reset Materials + Collision`
  (params (Opacity :type "Float (double-precision)"))
  ;[0.07812 0 1] If Back To 1 Opacity, switch back into original materials & use default collision (block cursor trace)
  (if (>= Opacity 1.0)
    (for (_array_element _array_index) (`self.Original Materials`)
      (`PrimitiveComponent.SetMaterial` (`self.Mesh`) _array_index _array_element))))

(event `Handle Collision`
  (params (Opacity :type "Float (double-precision)"))
  ;[0 0.0625 1] Handle Collision For Fade (Only Useful for objects like stairs which can be climbed on)
  (if (>= Opacity 1.0)
    (`PrimitiveComponent.SetCollisionResponseToChannel` (`self.Mesh`) "ECC_GameTraceChannel2" "ECR_Block")
    (if (`self.Should Block Visibility?`)
      (`PrimitiveComponent.SetCollisionResponseToChannel` (`self.Mesh`) "ECC_Visibility" "ECR_Block"))
    (elif (<= Opacity 0.05)
      (`PrimitiveComponent.SetCollisionResponseToChannel` (`self.Mesh`) "ECC_GameTraceChannel2" "ECR_Ignore")
      (if (`self.Should Block Visibility?`)
        (`PrimitiveComponent.SetCollisionResponseToChannel` (`self.Mesh`) "ECC_Visibility" "ECR_Ignore")))))

(fn `Set Materials To Dynamic Instances`
  (for (_array_element _array_index) (`self.Dynamic Material Instances`)
    (`PrimitiveComponent.SetMaterial` (`self.Mesh`) _array_index _array_element)))

(fn `UserConstructionScript`
  ;[0 1 0.5078] Store Original Materials and create dynamic mats from fade materials instances
  (`KismetArrayLibrary.Array_Clear` (`self.Dynamic Material Instances`))
  (set `self.Original Materials` (`MeshComponent.GetMaterials` (`self.Mesh`)))
  (for _array_element (`self.Fade Materials`)
    (bind _returnvalue (`KismetMaterialLibrary.CreateDynamicMaterialInstance` _array_element))
    (`KismetArrayLibrary.Array_AddUnique` (`self.Dynamic Material Instances`) _returnvalue)))