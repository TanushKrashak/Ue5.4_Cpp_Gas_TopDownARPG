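; BP_FlamePillar is a cosmetic world actor that makes a fire light flicker.
; On BeginPlay it randomly plays one of two intensity timelines at a random play rate, and picks again each time one finishes, looping indefinitely.
; Each timeline update sets FireLight intensity to the curve value multiplied by BaseIntensity, so the flicker varies without an obvious repeat.
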(event `self.ReceiveBeginPlay`
  (`self.Choose Random Timeline`))

(event `Start Flame Timeline 1`
  ;[1 0 0.5391] Flame Light Intensity Timelines
  (bind (_direction _flame_intensity) (`Timeline|Flame Light Intensity` :!via `PlayFromStart`)
    (:`Update`
      (`self.Set Flame Intensity` _flame_intensity))
    (:`Finished`
      (`self.Choose Random Timeline`))))

(event `Choose Random Timeline`
  ;[0 1 0.9297] Randomly Select Flame Timeline + Speed Of Flame Timeline
  (if (`KismetMathLibrary.RandomBool`)
    (`self.Start Flame Timeline 1`)
    (`TimelineComponent.SetPlayRate` (`self.Flame Light Intensity`) (`KismetMathLibrary.RandomFloatInRange` 0.3 0.7))
    (else
      (`self.Start Flame Timeline 2`)
      (`TimelineComponent.SetPlayRate` (`self.Flame Light Intensity 2`) (`KismetMathLibrary.RandomFloatInRange` 0.3 0.7)))))

(event `Start Flame Timeline 2`
  ;[1 0 0.5391] Flame Light Intensity Timelines
  (bind (_direction _flame_intensity) (`Timeline|Flame Light Intensity 2` :!via `PlayFromStart`)
    (:`Update`
      (`self.Set Flame Intensity` _flame_intensity))
    (:`Finished`
      (`self.Choose Random Timeline`))))

(fn `Set Flame Intensity`
  (params (`Intensity Multiplier` :type "Float (double-precision)"))
  (`LightComponent.SetIntensity` (`self.FireLight`) (* `Intensity Multiplier` (`self.Base Intensity`))))

(fn `UserConstructionScript`)