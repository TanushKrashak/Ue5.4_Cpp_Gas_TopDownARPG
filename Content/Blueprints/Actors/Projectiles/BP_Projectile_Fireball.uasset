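; Homing fireball projectile actor that explodes when the target it is chasing dies.
; On BeginPlay it delays enabling query-only sphere collision and applies a temporary ignore response on a custom trace channel, meant to stop same-owner projectiles colliding.
; Each Tick it asks the homing target's owner via an interface whether it is dead, then plays hit effects and destroys itself.
; An unused movement-distance check remains as an alternative.
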(event `self.ReceiveBeginPlay`
  ;[0.9688 0 1] This part is so that it doesn't collide with the floor or anything else on spawn (deprecated)
  (`|ExecutionSequence`
    (:`then_0`
      (`KismetSystemLibrary.Delay` 0.1)
      (bind _spherecomponent (`self.SphereComponent`)
        (:`then`
          (`PrimitiveComponent.SetCollisionEnabled` _spherecomponent "QueryOnly"))
        (:`else`)))
    (:`then_1`
      ;;[1 0.6563 0] TEMPORARY ONLY, DO REMOVE THIS AND ADD CUSTOM LOGIC FOR COLLISION HANDLING, SO THAT ALL OWNER PROJECTILS DO NOT HIT EACH OTHER
      (`PrimitiveComponent.SetCollisionResponseToChannel` (`self.SphereComponent`) "ECC_GameTraceChannel1" "ECR_Ignore")
      (`KismetSystemLibrary.Delay` 0.3)
      (`PrimitiveComponent.SetCollisionResponseToChannel` (`self.SphereComponent`) "ECC_GameTraceChannel1" "ECR_Ignore"))))

(event `self.ReceiveTick`
  (params (DeltaSeconds :type "Float (single-precision)"))
  ;[1 0 0.6328] Explode Fireball if its Homing Target Dies
  (bind _homingtargetcomponent (`ProjectileMovementComponent.HomingTargetComponent` (`self.ProjectileMovementComponent`))
    (:`then`
      (bind _returnvalue (message `Cpp_CombatInterface.IsDead` (`ActorComponent.GetOwner` _homingtargetcomponent)))
      (if _returnvalue
        (`self.OnHitEffects`)
        (`self.K2_DestroyActor`)))
    (:`else`)))

(fn `UserConstructionScript`)