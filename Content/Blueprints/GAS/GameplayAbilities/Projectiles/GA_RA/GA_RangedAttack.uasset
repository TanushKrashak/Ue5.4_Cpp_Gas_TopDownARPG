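; Gameplay ability for a ranged attack that fires a projectile at the avatar's combat target.
; On activation it picks a random tagged attack montage from the avatar, turns the avatar to face the target and plays the montage.
; The montage's gameplay event tag triggers the spawn from the matching socket, aimed at the target's current location plus an offset.
; The ability ends when the montage completes, is interrupted or is cancelled.
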(event `self.K2_ActivateAbility`
  (bind _returnvalue (`self.GetAvatarActorFromActorInfo`))
  ;[0.8281 1 0] Get Random Attack Montage
  (bind _returnvalue_2 (message `Cpp_CombatInterface.GetAttackMontages` (`self.GetAvatarActorFromActorInfo`)))
  (set `self.Randomly Chosen Tagged Montage` (`self.GetRandomTaggedMontageFromArray` _returnvalue_2))
  ;[0 0.0625 1] Set Enemy Location
  (bind _returnvalue_3 (message `Cpp_InteractionInterface.GetCombatTarget` _returnvalue))
  (message `Cpp_CombatInterface.SetFacingTargetLocation` _returnvalue (`Actor.K2_GetActorLocation` _returnvalue_3))
  (`AbilityTask_PlayMontageAndWait.CreatePlayMontageAndWaitProxy` "None" (`.Montage` (break `TaggedMontage` (`self.Randomly Chosen Tagged Montage`)))
    (:`then`
      ;[1 0 0.8203] On Attack Tag, get correct socket location and players within radius and cause dmg
      (`AbilityTask_WaitGameplayEvent.WaitGameplayEvent` (`.MontageTag` (break `TaggedMontage` (`self.Randomly Chosen Tagged Montage`))) null
        (:`EventReceived`
          (bind _returnvalue_4 (message `Cpp_InteractionInterface.GetCombatTarget` (`self.GetAvatarActorFromActorInfo`)))
          (`self.SpawnProjectile` (+ (`self.Projectile Target Offset`) (`Actor.K2_GetActorLocation` _returnvalue_4)) (`.SocketTag` (break `TaggedMontage` (`self.Randomly Chosen Tagged Montage`))) (`self.Override Pitch?`) (`self.Pitch Override`)))))
    (:`OnCompleted`
      (`self.K2_EndAbility` :!label _label))
    (:`OnInterrupted`
      (goto _label))
    (:`OnCancelled`
      (goto _label))))