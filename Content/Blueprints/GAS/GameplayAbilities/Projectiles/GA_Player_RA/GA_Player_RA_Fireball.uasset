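; Player fireball gameplay ability that casts projectiles toward the location under the mouse.
; Cursor target data supplies the location and hit actor, and the avatar turns to face that point before the ability commits cost and cooldown.
; The cast montage's gameplay event triggers SpawnProjectiles from the weapon socket, with an overridden pitch and the hit actor as homing target.
; The ability ends when the montage completes, blends out, or is interrupted or cancelled.
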(event `self.K2_ActivateAbility`
  ;[1 0.5625 0] Get Mouse Location for Target Location
  (bind (_asynctaskproxy _datahandle) (`Cpp_AT_TargetDataUnderMouse.CreateTargetDataUnderMouseTask`)
    (:`ValidData`
      (bind (_bblockinghit _binitialoverlap _time _distance _location _impactpoint _normal _impactnormal _physmat _hitactor) (`GameplayStatics.BreakHitResult` (`AbilitySystemBlueprintLibrary.GetHitResultFromTargetData` _datahandle)))
      (set `self.ProjectileTargetLocation` _location)
      (set `self.Hit Actor` _hitactor)
      (message `Cpp_CombatInterface.SetFacingTargetLocation` (`self.GetAvatarActorFromActorInfo`) (`self.ProjectileTargetLocation`))
      (`self.K2_CommitAbility`) ; This part checks for the currency\nas well as trhe cooldown
      (`AbilityTask_PlayMontageAndWait.CreatePlayMontageAndWaitProxy` "None" "/Game/Assets/Characters/Aura/Animations/Abilities/AM_Aura_Cast_Firebolt.AM_Aura_Cast_Firebolt" 1.0 "None" false
        (:`then`
          (`AbilityTask_WaitGameplayEvent.WaitGameplayEvent` (struct :`TagName` "Event.Montage.FireBolt") null
            (:`EventReceived`
              (`self.SpawnProjectiles` (`self.ProjectileTargetLocation`) (`BlueprintGameplayTagLibrary.MakeLiteralGameplayTag` (struct :`TagName` "CombatSocket.Weapon")) true 20.0 (`self.Hit Actor`)))))
        (:`OnCompleted`
          (`self.K2_EndAbility` :!label _label))
        (:`OnBlendOut`
          (goto _label))
        (:`OnInterrupted`
          (goto _label))
        (:`OnCancelled`
          (goto _label))))))