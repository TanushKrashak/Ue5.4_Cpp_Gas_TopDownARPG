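; Player Electrocute gameplay ability: a held channelled lightning attack on the target under the cursor that chains to additional targets.
; After motion warping, a montage event locks movement, adds looping shock cues and starts a timer that spends mana to damage every target.
; Input release (after a minimum hold), failed cost or primary target death ends it, committing cooldown.
; Cleanup applies a server-side final hit, so the debuff lands only once.
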(event `self.K2_ActivateAbility`
  (bind _damage_delta_time (`self.Damage Delta Time`))
  ;[0.6172 0 1] End Ability In Case owner does not implement Combat Interface
  (if (`KismetSystemLibrary.DoesImplementInterface` (`self.GetAvatarActorFromActorInfo`) "/Script/Aura.Cpp_CombatInterface")
    ;[0 0.6484 1] Store Cursor Data
    (bind (_asynctaskproxy _datahandle) (`Cpp_AT_TargetDataUnderMouse.CreateTargetDataUnderMouseTask`)
      (:`ValidData`
        (`self.StoreMouseData` (`AbilitySystemBlueprintLibrary.GetHitResultFromTargetData` _datahandle))
        ;[0 1 0.08594] Store Character + Controller and Hide Mouse
        (`self.StoreOwnerVariables`)
        (set `PlayerController.bShowMouseCursor` false (`self.OwnerPlayerController`))
        (`|ExecutionSequence`
          (:`then_0`
            (message `Cpp_CombatInterface.SetFacingTargetLocation` (`self.GetAvatarActorFromActorInfo`) (`self.MouseHitLocation`)) ; Motion Warping Target
            (`self.K2_ExecuteGameplayCue` (struct :`TagName` "GameplayCue.ShockBurst"))
            (`AbilityTask_PlayMontageAndWait.CreatePlayMontageAndWaitProxy` "None" (`self.Montage_Electrocute`) 1.0 "None" false
              (:`then`
                (`AbilityTask_WaitGameplayEvent.WaitGameplayEvent` (struct :`TagName` "Event.Montage.Electrocute") null true
                  (:`then`
                    ;[0 0.5547 1] Put it electrocute attack loop animation Store Primary Target
                    (message `Cpp_CombatInterface.SetInElectrocuteAttackLoop` (`self.GetAvatarActorFromActorInfo`) true)
                    (`self.TraceFirstTarget` (`self.MouseHitLocation`)))
                  (:`EventReceived`
                    ;[0 1 0.5078] Only Disable Movement after motion warping has finished
                    (`CharacterMovementComponent.DisableMovement` (`Character.CharacterMovement` (`self.OwnerCharacter`)))
                    ;[0 1 0.625] Spawn Cue
                    (`self.Spawn Looping Cue`)
                    (`self.Spawn Looping Cue For Additional Targets`)
                    ;[0.5 0 1] Damage Actor and use mana
                    (bind _returnvalue (`KismetSystemLibrary.K2_SetTimerDelegate` (`|CreateDelegate` :!event `Do Damage Using Cost`) _damage_delta_time true false (* _damage_delta_time -1.0)))
                    (set `self.Damage And Cost Timer` _returnvalue))))))
          (:`then_1`
            ;[0 0.3906 1] Once Input key released, prepare ending of ability and end it
            (bind (_asynctaskproxy_2 _timeheld) (`AbilityTask_WaitInputRelease.WaitInputRelease` false)
              (:`OnRelease`
                ;;[1 0 0.6797] This part let's the ability deal dmg atleast once
                (if (> _timeheld (`self.Min Time Held To Close Ability`))
                  (`self.Prepare To End Ability` :!label _label)
                  (`self.K2_EndAbility`)
                  (else
                    (`self.K2_HasAuthority` ; this should fix the issue wherein\nthe electricity for the electrocute\nstill stays even though the ability\nshould have ended properly, It was\na display only issue
                      (:`True`
                        (`KismetSystemLibrary.Delay` (- (`self.Min Time Held To Close Ability`) _timeheld))
                        (goto _label))
                      (:`False`
                        (`self.Prepare To End Ability`) ; Client's mouse cursor and other things\nshoudl atleast be shown, also clearing\nredundant variables
                      ))))))))))
    (else
      (`self.K2_EndAbility`))))

(event `Do Damage Using Cost`
  ;[1 0 0.1406 1 30] Do Damage Using Cost-  use mana and if not enough, end ability
  (bind _returnvalue (`self.K2_CommitAbilityCost` false))
  (if _returnvalue
    (`self.Apply Damage`)
    (else
      (`self.Prepare To End Ability`)
      (`self.K2_EndAbility`))))

(event `self.PrimaryTargetDied`
  (params (DeadActor :type "Actor Object Reference"))
  ;[0 1 0.2031 1 30] On Target Died
  (`GameplayCueFunctionLibrary.RemoveGameplayCueOnActor` DeadActor (struct :`TagName` "GameplayCue.ShockLoop") (`self.First Target Cue Params`))
  (`self.Prepare To End Ability`)
  (`self.K2_EndAbility`))

(event `self.AdditionalTargetDied`
  (params (DeadActor :type "Actor Object Reference"))
  ;[0 1 0.2031 1 30] On Target Died
  (`self.Remove Cue From Additional Target` DeadActor)
  (`BlueprintMapLibrary.Map_Remove` (`self.Additioal Actors To Cue Params`) DeadActor))

(fn `Apply Damage`
  (`self.Apply Damage to Single Actor` (`self.MouseHitActor`))
  ;[0.5937 1 0] Applying damage to chained electrocute people
  (bind _keys (`BlueprintMapLibrary.Map_Keys` (`self.Additioal Actors To Cue Params`)))
  (for _array_element _keys
    (`self.Apply Damage to Single Actor` _array_element)))

(fn `Apply Damage to Single Actor`
  (params (Actor :type "Actor Object Reference"))
  (bind _returnvalue (`self.GetAbilitySystemComponentFromActorInfo`))
  (bind _returnvalue_2 (`AbilitySystemBlueprintLibrary.GetAbilitySystemComponent` (`local.Actor`)))
  (`/Engine/EditorBlueprintResources/StandardMacros.IsValid` Actor
    (:`Is Valid`
      (`/Engine/EditorBlueprintResources/StandardMacros.IsValid` _returnvalue
        (:`Is Valid`
          (bind _returnvalue_3 (`AbilitySystemBlueprintLibrary.AssignTagSetByCallerMagnitude` (`AbilitySystemComponent.MakeOutgoingSpec` _returnvalue (`self.DamageEffectClass`) (`KismetMathLibrary.Conv_IntToDouble` (`self.GetAbilityLevel`)) (`AbilitySystemComponent.MakeEffectContext` _returnvalue)) (`self.DamageType`) (`self.GetDamageBasedOnLevel`)))
          (`/Engine/EditorBlueprintResources/StandardMacros.IsValid` _returnvalue_2
            (:`Is Valid`
              (`AbilitySystemComponent.BP_ApplyGameplayEffectSpecToSelf` _returnvalue_2 _returnvalue_3))))))))

(fn `Prepare To End Ability`
  (`self.K2_CommitAbilityCooldown` false)
  (`KismetSystemLibrary.K2_ClearAndInvalidateTimerHandle` (`self.Damage And Cost Timer`))
  (set `PlayerController.bShowMouseCursor` true (`self.OwnerPlayerController`))
  ;[0.1016 1 0] Remove from electocute Loop + Enable Movement + Remove Loop Cue
  (message `Cpp_CombatInterface.SetInElectrocuteAttackLoop` (`self.GetAvatarActorFromActorInfo`) false)
  (`CharacterMovementComponent.SetMovementMode` (`Character.CharacterMovement` (`self.OwnerCharacter`)) "MOVE_Walking" 0)
  (`GameplayCueFunctionLibrary.RemoveGameplayCueOnActor` (select `bool` (`self.Hit Actor Implements Combat Interface?`) :`false` (`self.OwnerCharacter`) :`true` (`self.MouseHitActor`) :!type "Actor Object Reference") (struct :`TagName` "GameplayCue.ShockLoop") (`self.First Target Cue Params`))
  ;[1 0 0.3281] Reset Variables
  (if (`self.Hit Actor Implements Combat Interface?`)
    (`self.K2_HasAuthority`
      (:`True`
        (`Cpp_BFL_AbilitySystem.ApplyDamageEffectWithDamageParams` (`self.MakeDamageEffectParamsFromClassDefaults` (`self.MouseHitActor`))) ; Does the last hit, which gives the debuff effect\nthis is done so that the debuff effect isn't applied\non each electrocute hit, but on the last, so the \nenemy stays stunned after the electrocute attack\nhas completed
      )
      (:`False`
        _))
    (message `Cpp_CombatInterface.SetIsBeingShocked` (`self.MouseHitActor`) false)
    (bind _keys (`BlueprintMapLibrary.Map_Keys` (`self.Additioal Actors To Cue Params`)))
    (for _array_element _keys
      (`self.Remove Cue From Additional Target` _array_element)
      (message `Cpp_CombatInterface.SetIsBeingShocked` _array_element false)
      (`self.K2_HasAuthority`
        (:`True`
          (`Cpp_BFL_AbilitySystem.ApplyDamageEffectWithDamageParams` (`self.MakeDamageEffectParamsFromClassDefaults` _array_element)) ; Does the last hit, which gives the debuff effect\nthis is done so that the debuff effect isn't applied\non each electrocute hit, but on the last, so the \nenemy stays stunned after the electrocute attack\nhas completed
        ))))
  (`BlueprintMapLibrary.Map_Clear` (`self.Additioal Actors To Cue Params`))
  (set `self.MouseHitActor` null)
  (set `self.Hit Actor Implements Combat Interface?` false))

(fn `Remove Cue From Additional Target`
  (params (Actor :type "Actor Object Reference (by ref)"))
  (`GameplayCueFunctionLibrary.RemoveGameplayCueOnActor` Actor (struct :`TagName` "GameplayCue.ShockLoop") (`BlueprintMapLibrary.Map_Find` (`self.Additioal Actors To Cue Params`) Actor)))

(fn `Spawn Looping Cue`
  (locals (`Cue Target` :type "Actor Object Reference"))
  (bind _returnvalue (`KismetSystemLibrary.DoesImplementInterface` (`self.MouseHitActor`) "/Script/Aura.Cpp_CombatInterface"))
  (bind _returnvalue_2 (message `Cpp_CombatInterface.GetWeapon` (`self.GetAvatarActorFromActorInfo`)))
  (set `self.First Target Cue Params` (`AbilitySystemBlueprintLibrary.MakeGameplayCueParameters` 0.0 0.0 (struct) (struct) (struct) (struct) (struct) (`self.MouseHitLocation`) (0.0 0.0 0.0) null null (`self.MouseHitActor`) null 1 1 _returnvalue_2))
  (set `self.Hit Actor Implements Combat Interface?` _returnvalue)
  (set `local.Cue Target` (select `bool` _returnvalue :`false` (`self.GetAvatarActorFromActorInfo`) :`true` (`self.MouseHitActor`))) ; Is Mouse Hit Actor An Enemy?\nIf yes then Set it to Hit Actor\nif no, then set it to owner / \nAvatar Actor
  (`GameplayCueFunctionLibrary.AddGameplayCueOnActor` (`local.Cue Target`) (struct :`TagName` "GameplayCue.ShockLoop") (`self.First Target Cue Params`)))

(fn `Spawn Looping Cue For Additional Targets`
  (locals (Target :type "Actor Object Reference"))
  (bind _target (`local.Target`))
  (bind _returnvalue (`AbilitySystemBlueprintLibrary.MakeGameplayCueParameters` 0.0 0.0 (struct) (struct) (struct) (struct) (struct) (`Actor.K2_GetActorLocation` _target) (0.0 0.0 0.0) null null _target null 1 1 (`Actor.RootComponent` (`self.MouseHitActor`))))
  ;[1 0 0.6328 1 30] Spawn Chain Lightning Cues For Nearby Enemies, Only if the target was an enemy and not an object
  (if (`self.Hit Actor Implements Combat Interface?`)
    (message `Cpp_CombatInterface.SetIsBeingShocked` (`self.MouseHitActor`) true)
    (bind _outadditionaltargets (`self.FindAndStoreAdditionalTargets`))
    (for _array_element _outadditionaltargets
      (set `local.Target` _array_element)
      (message `Cpp_CombatInterface.SetIsBeingShocked` _array_element true)
      (`BlueprintMapLibrary.Map_Add` (`self.Additioal Actors To Cue Params`) (`local.Target`) _returnvalue)
      (`GameplayCueFunctionLibrary.AddGameplayCueOnActor` (`local.Target`) (struct :`TagName` "GameplayCue.ShockLoop") _returnvalue))))