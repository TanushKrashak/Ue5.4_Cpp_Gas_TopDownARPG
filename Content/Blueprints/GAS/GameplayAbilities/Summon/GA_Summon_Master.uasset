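; Master summon Gameplay Ability that turns the avatar toward its combat target and plays the Shaman summon montage.
; Shortly after the montage starts, it shuffles the spawn locations and marks each with a Niagara ground effect.
; A montage gameplay event starts a delayed DoN loop that spawns a random class at each location, facing away from the avatar.
; Each spawn raises the avatar's summon count, and its destruction lowers it.
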(event `self.K2_ActivateAbility`
  (bind _returnvalue (`self.GetAvatarActorFromActorInfo`))
  ;[0 0.0625 1] Set Enemy Location
  (bind _returnvalue_2 (message `Cpp_InteractionInterface.GetCombatTarget` _returnvalue))
  (message `Cpp_CombatInterface.SetFacingTargetLocation` _returnvalue (`Actor.K2_GetActorLocation` _returnvalue_2))
  (`AbilityTask_PlayMontageAndWait.CreatePlayMontageAndWaitProxy` "None" "/Game/Assets/Enemies/Shaman/Animations/AM_Shaman_Summon.AM_Shaman_Summon"
    (:`then`
      (`AbilityTask_WaitGameplayEvent.WaitGameplayEvent` (struct :`TagName` "Montage.Attack.1") null
        (:`then`
          (`KismetSystemLibrary.Delay` 0.5)
          ;[0.9453 1 0] Get Spawn Locations
          (bind _returnvalue_3 (`self.GetSpawnLocations`))
          (bind _output_get (set `self.Spawn Locations` _returnvalue_3))
          (`KismetArrayLibrary.Array_Shuffle` _output_get)
          ;[0 1 0.1094] Pre Enemy Spawning Location Indicators
          (for _array_element (`self.Spawn Locations`)
            (`NiagaraFunctionLibrary.SpawnSystemAtLocation` "/Game/Assets/Effects/Combat/NS_GroundSummon.NS_GroundSummon" _array_element)))
        (:`EventReceived`
          ;[1 0 0.2344] Delayed Enemy Spawning
          (bind _counter (`/Engine/EditorBlueprintResources/StandardMacros.Do N` (`KismetArrayLibrary.Array_Length` (`self.Spawn Locations`)) :!label _label)
            (:`Exit`
              (bind _returnvalue_4 (+ (`|GetArrayItem` (`self.Spawn Locations`) (- _counter 1)) (0.0 0.0 75.0)))
              (bind _returnvalue_5 (`|SpawnActorFromClass` (`self.GetRandomSpawnClass`) (`KismetMathLibrary.MakeTransform` _returnvalue_4 (`KismetMathLibrary.FindLookAtRotation` (`Actor.K2_GetActorLocation` (`self.GetAvatarActorFromActorInfo`)) _returnvalue_4)) "AdjustIfPossibleButAlwaysSpawn" "MultiplyWithRoot" null null))
              (add `Actor.OnDestroyed` _returnvalue_5 (`|CreateDelegate` :!event `Decrement Summon Count`))
              (message `Cpp_CombatInterface.UpdateSummonsCount` (`self.GetAvatarActorFromActorInfo`) 1)
              (`KismetSystemLibrary.Delay` 0.5)
              (goto _label))))))))

(event `Decrement Summon Count`
  (params (DestroyedActor :type "Actor Object Reference"))
  ;[0 1 0.4844 1 30] Decrement Summon Count When Summon Dies
  (message `Cpp_CombatInterface.UpdateSummonsCount` (`self.GetAvatarActorFromActorInfo`) -1))