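; GA_MeleeAttack is a melee attack gameplay ability that faces the avatar toward its combat target and plays a random tagged attack montage.
; The montage's gameplay event triggers a small-radius search for living players around the tagged socket.
; Non-friendly hits take damage through class-default damage effect params, which carry extras like knockback.
; Any hit fires a MeleeImpact gameplay cue, and the ability ends when the montage completes, is interrupted or is cancelled.
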(event `self.K2_ActivateAbility`
  (bind _returnvalue (`self.GetAvatarActorFromActorInfo`))
  (bind _returnvalue_2 (`self.GetAvatarActorFromActorInfo`))
  (bind ((`MontageTag` _montagetag) (`SocketTag` _sockettag)) (break `TaggedMontage` (`self.Randomly Chosen TaggedMontage`)))
  ;[0 0.2734 1] Reset Values
  (set `self.HasHitTarget?` false)
  ;[1 0 0.7266] Get Random Attack Montage
  (bind _returnvalue_3 (message `Cpp_CombatInterface.GetAttackMontages` (`self.GetAvatarActorFromActorInfo`)))
  (set `self.Randomly Chosen TaggedMontage` (`self.GetRandomTaggedMontageFromArray` _returnvalue_3))
  ;[0 0.0625 1] Set Enemy Location
  (bind _returnvalue_4 (message `Cpp_InteractionInterface.GetCombatTarget` _returnvalue_2))
  (message `Cpp_CombatInterface.SetFacingTargetLocation` _returnvalue_2 (`Actor.K2_GetActorLocation` _returnvalue_4))
  (`AbilityTask_PlayMontageAndWait.CreatePlayMontageAndWaitProxy` "None" (`.Montage` (break `TaggedMontage` (`self.Randomly Chosen TaggedMontage`)))
    (:`then`
      ;[1 0 0.8203 1 30] On Attack Tag, get correct socket location and players within radius and cause dmg
      (`AbilityTask_WaitGameplayEvent.WaitGameplayEvent` _montagetag null
        (:`EventReceived`
          (bind _returnvalue_5 (message `Cpp_CombatInterface.GetSocketLocation` _returnvalue _sockettag))
          (bind _output_get (set `self.Socket Location` _returnvalue_5))
          (bind _outactors (`Cpp_BFL_AbilitySystem.GetAlivePlayersWithinRadius` self (`|MakeArray` _returnvalue) _output_get 45.0))
          (for _array_element _outactors
            ;;[0.4297 0 1] If Hostile, Deal Damage
            (if (`Cpp_BFL_AbilitySystem.IsNotFriend` _array_element (`self.GetAvatarActorFromActorInfo`))
              (`Cpp_BFL_AbilitySystem.ApplyDamageEffectWithDamageParams` (`self.MakeDamageEffectParamsFromClassDefaults` _array_element)) ; Using this instead of the Cause Damage node\ncuz this has other properties which are set, like\nknockback
              (set `self.HasHitTarget?` true)))
          ;;[0.2188 0 1] Play Hit Sound & Niagra Effect
          (if (`self.HasHitTarget?`)
            (bind _returnvalue_6 (message `Cpp_InteractionInterface.GetCombatTarget` (`self.GetAvatarActorFromActorInfo`)))
            (`self.K2_ExecuteGameplayCueWithParams` (struct :`TagName` "GameplayCue.MeleeImpact") (`AbilitySystemBlueprintLibrary.MakeGameplayCueParameters` 0.0 0.0 (struct) (struct) (struct) (`BlueprintGameplayTagLibrary.MakeGameplayTagContainerFromTag` (`.MontageTag` (break `TaggedMontage` (`self.Randomly Chosen TaggedMontage`)))) (struct) (`self.Socket Location`) (0.0 0.0 0.0) null (`self.GetAvatarActorFromActorInfo`) _returnvalue_6))))))
    (:`OnCompleted`
      (`self.K2_EndAbility` :!label _label))
    (:`OnInterrupted`
      (goto _label))
    (:`OnCancelled`
      (goto _label))))