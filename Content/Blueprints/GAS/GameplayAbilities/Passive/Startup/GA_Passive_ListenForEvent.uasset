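; Passive Gameplay Ability that listens for any gameplay event under the Attributes tag and turns it into a Gameplay Effect on its owner.
; Each event's magnitude serves as the effect spec's level and as the SetByCaller value for the exactly matching tag in EventTags.
; All other listed tags are set to zero, so one shared effect class changes only that attribute when applied to self.
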(event `self.K2_ActivateAbility`
  (bind _returnvalue (`self.GetAbilitySystemComponentFromActorInfo`))
  (bind (_asynctaskproxy _payload) (`AbilityTask_WaitGameplayEvent.WaitGameplayEvent` (struct :`TagName` "Attributes") null false false) ; Fire if any attribute was changed
    (:`EventReceived`
      (bind ((`EventTag` _eventtag) (`EventMagnitude` _eventmagnitude)) (break `GameplayEventData` _payload))
      ;[1 0 0.3984] Store Tag + Magnitude + Outgoing Spec
      (set `self.Temporary Event Tag` _eventtag)
      (bind _output_get (set `self.Temporary Event Magnitude` _eventmagnitude))
      (set `self.Temporary Outgoing Spec` (`AbilitySystemComponent.MakeOutgoingSpec` _returnvalue (`self.Even Based Effect Class`) _output_get (`AbilitySystemComponent.MakeEffectContext` _returnvalue)))
      ;[0.6875 0 1] Go Through all Tags, If Match, then do its effect, otherwise set rest to 0 magnitude (no change for them) and finally  apply it to self
      (for _array_element (`self.Event Tags`)
        (if (`BlueprintGameplayTagLibrary.MatchesTag` _array_element (`self.Temporary Event Tag`) true)
          (`AbilitySystemBlueprintLibrary.AssignTagSetByCallerMagnitude` (`self.Temporary Outgoing Spec`) (`self.Temporary Event Tag`) (`self.Temporary Event Magnitude`))
          (else
            (`AbilitySystemBlueprintLibrary.AssignTagSetByCallerMagnitude` (`self.Temporary Outgoing Spec`) _array_element))))
      (`AbilitySystemComponent.BP_ApplyGameplayEffectSpecToSelf` (`self.GetAbilitySystemComponentFromActorInfo`) (`self.Temporary Outgoing Spec`)))))