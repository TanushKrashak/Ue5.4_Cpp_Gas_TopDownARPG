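; BP_Enemy_Master is the enemy master Blueprint, handling spawn, dissolve and facing visuals.
; BeginPlay calls the parent, then a timeline drives mesh scale as a spawn effect.
; Two dissolve events each play a timeline that writes the Dissolve scalar on a supplied dynamic material, for mesh and weapon.
; SetFacingTargetLocation updates the FacingTarget motion-warping target from a given location.
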(event `self.StartDissolveTimeline`
  (params (DynamicMaterialInstance :type "MaterialInstanceDynamic Object Reference"))
  ;[1 0.9844 0] Dissolve Mesh + Weapon
  (bind (_direction _dissolve_track) (`Timeline|Dissolve Timeline` :!via `PlayFromStart`)
    (:`Update`
      (`MaterialInstanceDynamic.SetScalarParameterValue` DynamicMaterialInstance "Dissolve" _dissolve_track))))

(event `self.StartWeaponDissolveTimeline`
  (params (DynamicMaterialInstance :type "MaterialInstanceDynamic Object Reference"))
  ;[1 0.9844 0] Dissolve Mesh + Weapon
  (bind (_direction _dissolve_track) (`Timeline|Timeline` :!via `PlayFromStart`)
    (:`Update`
      (`MaterialInstanceDynamic.SetScalarParameterValue` DynamicMaterialInstance "Dissolve" _dissolve_track))))

(event `self.SetFacingTargetLocation`
  (params (TargetLocation :type "Vector Structure (by ref)"))
  ;[0 0.9297 1] Update Facing Target Location For Motion Warping
  (`MotionWarpingComponent.AddOrUpdateWarpTargetFromLocation` (`self.MotionWarping`) "FacingTarget" TargetLocation))

(event `self.ReceiveBeginPlay`
  ;[0.3828 0 1] Event Beginplay
  (`parent.ReceiveBeginPlay`)
  ;;[1 0 0.8437] Give enemies a fancy spawning effect
  (bind (_direction _scale_track) (`Timeline|Spawn Timeline`)
    (:`Update`
      (`SceneComponent.SetRelativeScale3D` (`self.Mesh`) (`KismetMathLibrary.Conv_DoubleToVector` _scale_track)))))

(fn `UserConstructionScript`)