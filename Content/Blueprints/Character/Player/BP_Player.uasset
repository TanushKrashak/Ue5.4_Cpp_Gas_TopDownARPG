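; BP_Player is the player character Blueprint, handling camera occlusion fading, attack facing and a debug slow motion key.
; A FadeBox overlap sends fade out and fade in messages to actors that come between the camera and player.
; SetFacingTargetLocation updates the FacingTarget motion warping target, and a setter tracks the electrocute attack loop state.
; Holding Tab drops global time dilation to slow motion until release.
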(event OnComponentBeginOverlap(FadeBox)
  (params (OverlappedComponent :type Primitive%20Component%20Object%20Reference) (OtherActor :type Actor%20Object%20Reference) (OtherComp :type Primitive%20Component%20Object%20Reference) (OtherBodyIndex :type Integer) (bFromSweep :type Boolean) (SweepResult :type Hit%20Result%20Structure%20%28by%20ref%29))
  ;[0 0.625 1] Fade Out / In Other Actors If they come in between camera and player
  (Class|BPIFade|FadeOut(Message) OtherActor))

(event OnComponentEndOverlap(FadeBox)
  (params (OverlappedComponent :type Primitive%20Component%20Object%20Reference) (OtherActor :type Actor%20Object%20Reference) (OtherComp :type Primitive%20Component%20Object%20Reference) (OtherBodyIndex :type Integer))
  ;[0 0.625 1] Fade Out / In Other Actors If they come in between camera and player
  (Class|BPIFade|Fadein(Message) OtherActor))

(event Input|KeyboardEvents|DebugKeyTab
  (params (Key :type Key%20Structure :default "None") (ActionValue :type Input%20Action%20Value%20Structure))
  (:Pressed
    (Utilities|Time|SetGlobalTimeDilation 0.05))
  (:Released
    (Utilities|Time|SetGlobalTimeDilation 1.0)))

(event EventSetFacingTargetLocation
  (params (TargetLocation :type Vector%20%28by%20ref%29 :default "0, 0, 0"))
  ;[0 0.9297 1] Update Facing Target Location For Motion Warping
  (Class|MotionWarpingComponent|AddorUpdateWarpTargetfromLocation (Variables|Default|GetMotionWarping) "FacingTarget" TargetLocation))

(event EventSetinElectrocuteAttackLoop
  (params (bInLoop :type Boolean))
  (Variables|Animations|SetIn%20Electrocute%20Attack%20Loop? bInLoop))

(fn ConstructionScript)